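; BP_Bird is an actor that travels along the spline of a referenced track actor.
; On BeginPlay, if ActivateBird is set, MoveCart plays a timeline with its play rate scaled by the inverse of Duration.
; Each update maps the timeline alpha to a distance along the spline and sets the bird's world location and rotation from that point.
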(event Custom|MoveCart
  (Components|Timeline|SetPlayRate (Variables|Default|GetTimeline) (/ 1.0 (Variables|Default|GetDuration)))
  (bind _alpha (Timeline|Timeline Play)
    (:Update
      (Variables|Default|SetAlpha _alpha)
      (Transformation|SetActorLocationAndRotation (Spline|GetLocationatDistanceAlongSpline (Variables|/Game/Blueprints/SplineMovement/BP_Track.BP_Track_C|GetSpline (Variables|Default|GetTrackRef)) (Math|Float|Lerp 0.0 (Spline|GetSplineLength (Variables|/Game/Blueprints/SplineMovement/BP_Track.BP_Track_C|GetSpline (Variables|Default|GetTrackRef))) (Variables|Default|GetAlpha)) "World") (Spline|GetRotationatDistanceAlongSpline (Variables|/Game/Blueprints/SplineMovement/BP_Track.BP_Track_C|GetSpline (Variables|Default|GetTrackRef)) (Math|Float|Lerp 0.0 (Spline|GetSplineLength (Variables|/Game/Blueprints/SplineMovement/BP_Track.BP_Track_C|GetSpline (Variables|Default|GetTrackRef))) (Variables|Default|GetAlpha)) "World")))))

(event EventBeginPlay
  (if (Variables|Default|GetActivateBird)
    (CallFunction|MoveCart)))

(fn ConstructionScript)