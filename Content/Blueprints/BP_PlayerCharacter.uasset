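; Player character with movement, pause menu, a wind power claimed from an activated ability orb, and a toggleable Intuition vision mode.
; Holding the ability charges a cooldown-gated gust; charged shots push harder and recoil the player.
; Wind box-traces physics objects for impulses and line-traces puzzle actors.
; Intuition drives a material parameter collection, post-process settings, dispatchers and directional light, respecting cave state; both abilities dismiss tutorial hints.
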(event EventBeginPlay
  (Variables|Default|Setwalk_speed_ (Variables|/Script/Engine.CharacterMovementComponent|GetMaxWalkSpeed (Variables|Character|GetCharacterMovement)))
  (bind _returnvalue (Actor|GetActorOfClass "/Script/Engine.PostProcessVolume"))
  (Variables|Default|Setpostprocessiong_volume_ _returnvalue)
  (Variables|Default|SetTags (Variables|Default|GetPlayerTags))
  (bind _returnvalue_2 (Actor|GetActorOfClass "/Script/Engine.DirectionalLight"))
  (Variables|Default|Setdirectional_light_ _returnvalue_2))

(event EventTick
  (params (DeltaSeconds :type Float%20%28single-precision%29))
  (CallFunction|UpdateWindCD DeltaSeconds)
  (if (Variables|Default|Getwind_input_down_)
    (if (Variables|Default|Getwind_ready_)
      (Variables|Default|Setwind_hold_time_ (+ (Variables|Default|Getwind_hold_time_) DeltaSeconds)))))

(event Input|ActionEvents|InputActionJump
  (params (Key :type Key%20Structure :default "None"))
  ;[1 1 1] Movement and Camera
  (:Pressed
    (Character|Jump))
  (:Released
    (Character|StopJumping)))

(event Input|ActionEvents|InputActionIntuition
  (params (Key :type Key%20Structure :default "None"))
  (bind _directional_light_ (Variables|Default|Getdirectional_light_))
  (bind _in_cave_ (Variables|Default|Getin_cave_))
  (bind _player_ui (Variables|Default|GetPlayer%20UI))
  (bind _postprocessiong_volume_ (Variables|Default|Getpostprocessiong_volume_))
  (bind _settings (Variables|/Script/Engine.PostProcessVolume|GetSettings _postprocessiong_volume_))
  (bind _lightcomponent (Variables|/Script/Engine.Light|GetLightComponent _directional_light_))
  ;[0.436 1 0.9602] Toggle Intuition mode
  (:Pressed
    (if (Variables|Default|Getintuition_unlocked_)
      (if (Variables|Default|Getintuition_tutorial_)
        (if (Variables|Default|Getfirst_intuition_use_)
          (Default|HideIntuitionHInt _player_ui)
          (Variables|Default|Setfirst_intuition_use_ false)
          (else
            (Default|HideIntuitionExplanation _player_ui)
            (Variables|Default|Setintuition_tutorial_ false)))))
    (bind _output_get (Variables|Default|Setintuition_mode_ (not (Variables|Default|Getintuition_mode_))))
    (Rendering|Material|SetScalarParameterValue "/Game/VFX/Intuitionmode/MP_Intuitionmode.MP_Intuitionmode" "Intuitionmode_blend" (Math|Conversions|ToFloat(Boolean) _output_get) :!class /Script/Engine.KismetMaterialLibrary)
    (if (Math|Boolean|Equal(Boolean) (Variables|Default|Getintuition_mode_) true)
      (Default|CallIntuitiononEventDispatcher)
      (Utilities|Struct|SetmembersinPostProcessSettings _settings 5.0 0.5 0.5)
      (Audio|PlaySound2D "/Game/Audio/Ambient/Intuition_3_Entering.Intuition_3_Entering" 1.0 1.0 0.0 0 0)
      (if (not _in_cave_)
        (Rendering|Components|Light|SetIntensity _lightcomponent 0.0))
      (else
        (Default|CallIntuitionOffEventDispatcher)
        (Utilities|Struct|SetmembersinPostProcessSettings _settings 0.0 0.0 0.0)
        (Audio|PlaySound2D "/Game/Audio/Ambient/Intuition_3_Leaving.Intuition_3_Leaving" 1.0 1.0 0.0 0 0)
        (if (not _in_cave_)
          (Rendering|Components|Light|SetIntensity _lightcomponent (Variables|Default|Getoriginal_intensity_)))))))

(event Input|ActionEvents|InputActionRun
  (params (Key :type Key%20Structure :default "None"))
  (bind _charactermovement (Variables|Character|GetCharacterMovement))
  ;[1 1 1] Movement and Camera
  (:Pressed
    (Variables|/Script/Engine.CharacterMovementComponent|SetMaxWalkSpeed _charactermovement (Variables|Default|Getrun_speed_)))
  (:Released
    (Variables|/Script/Engine.CharacterMovementComponent|SetMaxWalkSpeed _charactermovement (Variables|Default|Getwalk_speed_))))

(event Input|ActionEvents|InputActionUseAbility
  (params (Key :type Key%20Structure :default "None"))
  (:Pressed
    (if (Variables|Default|Gethave_wind_power_)
      (Variables|Default|Setwind_input_down_ true)
      (if (Variables|Default|Getwind_ready_)
        (Audio|Components|Audio|Play (Variables|Default|GetAudio) 0.0))
      (else
        (CallFunction|GetWindPower))))
  (:Released
    (if (Variables|Default|Gethave_wind_power_)
      (CallFunction|Wind)
      (Variables|Default|Setwind_input_down_ false)
      (Variables|Default|Setwind_hold_time_ 0.0))))

(event Input|ActionEvents|InputActionPauseMenu
  (params (Key :type Key%20Structure :default "None"))
  (bind _returnvalue (Game|GetPlayerController 0))
  ;[0.8986 1 0.1365] PauseMenu
  (:Pressed
    (bind _returnvalue_2 (UserInterface|CreateWidget "/Game/UI/PauseMenu.PauseMenu_C"))
    (UserInterface|Viewport|AddtoViewport _returnvalue_2 0)
    (Input|SetInputModeUIOnly _returnvalue 0 "LockAlways")
    (Variables|/Script/Engine.PlayerController|SetbShowMouseCursor _returnvalue true)))

(event Input|AxisEvents|InputAxisMoveForward
  (params (AxisValue :type Float%20%28single-precision%29))
  ;[1 1 1] Movement and Camera
  (Pawn|Input|AddMovementInput (Transformation|GetActorForwardVector) AxisValue false))

(event Input|AxisEvents|InputAxisMoveRight
  (params (AxisValue :type Float%20%28single-precision%29))
  ;[1 1 1] Movement and Camera
  (Pawn|Input|AddMovementInput (Transformation|GetActorRightVector) AxisValue false))

(event Input|AxisEvents|InputAxisLookUp
  (params (AxisValue :type Float%20%28single-precision%29))
  ;[1 1 1] Movement and Camera
  (Pawn|Input|AddControllerPitchInput (* AxisValue (Variables|Default|GetSensitivity))))

(event Input|AxisEvents|InputAxisTurn
  (params (AxisValue :type Float%20%28single-precision%29))
  ;[1 1 1] Movement and Camera
  (Pawn|Input|AddControllerYawInput (* AxisValue (Variables|Default|GetSensitivity))))

(fn ConstructionScript)

(fn Wind
  (bind _camera (Variables|Default|GetCamera))
  (bind _capsulecomponent (Variables|Collision|GetCapsuleComponent))
  (bind _camera_2 (Variables|Default|GetCamera))
  (bind _camera_3 (Variables|Default|GetCamera))
  (bind _returnvalue (Transformation|GetWorldLocation _camera_2))
  (bind _returnvalue_2 (Transformation|GetWorldLocation _camera_3))
  (bind _returnvalue_3 (Transformation|GetWorldRotation _capsulecomponent))
  (bind _returnvalue_4 (Transformation|GetWorldLocation _camera))
  (bind _returnvalue_5 (Transformation|GetWorldRotation _camera_2))
  (bind _returnvalue_6 (Math|Rotator|MakeRotator (.roll _returnvalue_5) (.pitch _returnvalue_5) (.yaw _returnvalue_3)))
  (if (Variables|Default|Getwind_ready_)
    (Audio|Components|Audio|Stop (Variables|Default|GetAudio))
    (Variables|Default|Setwind_ready_ false)
    (Utilities|FlowControl|Sequence
      (:then_0
        (if (>= (Variables|Default|Getwind_hold_time_) 0.3)
          (Variables|Default|Setwind_force_ (Variables|Default|Getstrong_wind_force_))
          (Variables|Default|Setcharged_ true)
          (else
            (Variables|Default|Setwind_force_ (Variables|Default|Getlight_wind_force_))
            (Variables|Default|Setcharged_ false))))
      (:then_1
        ;[1 1 1] pushes all objects in front once
        (Game|SpawnActorfromClass "/Game/Blueprints/Wind/BP_Windvisual.BP_Windvisual_C" (Math|Transform|MakeTransform _returnvalue _returnvalue_6 "1,1,1") "Undefined" 0 0)
        (bind _returnvalue_7 (Game|SpawnActorfromClass "/Game/Blueprints/Wind/BP_WindVFX.BP_WindVFX_C" (Math|Transform|MakeTransform _returnvalue _returnvalue_6 "1,1,1") "Undefined" 0 0))
        (Default|SetVFX _returnvalue_7 (Variables|Default|Getcharged_))
        (bind (_outhits _returnvalue_8) (Class|KismetSystemLibrary|BoxTraceMultiforObjects _returnvalue (+ _returnvalue (* (Math|Vector|GetForwardVector _camera_2) (Variables|Default|Getwind_range_))) "100.000000,100.000000,100.000000" "0, 0, 0" (Utilities|Array|MakeArray "ObjectTypeQuery1" "ObjectTypeQuery3" "ObjectTypeQuery4") false 0 "None" true))
        (if _returnvalue_8
          (for _array_element _outhits
            (if (Physics|IsSimulatingPhysics (.HitComponent (Collision|BreakHitResult _array_element)) "None")
              (Physics|AddRadialImpulse (.HitComponent (Collision|BreakHitResult _array_element)) (Transformation|GetActorLocation) 5e+03 (Variables|Default|Getwind_force_) "RIF_Constant" true)
              (bind _asbp_pillar_wisp (Utilities|Casting|CastToBP_PillarWisp (.HitActor (Collision|BreakHitResult _array_element))))
              (Default|OnHit _asbp_pillar_wisp)))))
      (:then_2
        ;[1 1 1] Music pipe and pillar puzzle
        (bind _outhit (Collision|LineTraceByChannel _returnvalue_2 (+ _returnvalue_2 (* (Math|Vector|GetForwardVector _camera_3) (Variables|Default|Getwind_range_))) "TraceTypeQuery1" false 0 "None"))
        (Utilities|FlowControl|Sequence
          (:then_0
            (bind _asbp_music_pipe (Utilities|Casting|CastToBP_MusicPipe (.hitactor _outhit)))
            (Default|OnHit _asbp_music_pipe))
          (:then_1
            (bind _asbp_pillar_puzzle (Utilities|Casting|CastToBP_PillarPuzzle (.hitactor _outhit)))
            (if (Variables|/Game/Blueprints/PillarPuzzle/BP_PillarPuzzle.BP_PillarPuzzle_C|Getdone_ _asbp_pillar_puzzle)
              (Default|Finish _asbp_pillar_puzzle)))))
      (:then_3
        ;[1 1 1] Play Wind Sound
        (if true
          (Audio|PlaySoundatLocation (Variables|Default|Getwind_power_sound__charged_) _returnvalue_4 "0, 0, 0" 1.0 1.0 0.0 0 0 0)
          (else
            (Audio|PlaySoundatLocation (Variables|Default|Getwind_power_sound_) _returnvalue_4 "0, 0, 0" 1.0 1.0 0.0 0 0 0))))
      (:then_4
        (if (Variables|Default|Getcharged_)
          (Character|LaunchCharacter self (* (* (Math|Vector|GetForwardVector (Transformation|GetWorldRotation (Variables|Default|GetCamera))) -1.0) (Variables|Default|Getwind_recoil)) false false)))
      (:then_5
        (if (Variables|Default|Getfirst_charge_use)
          (if (Variables|Default|Getfirst_use_)
            (if (not (Variables|Default|Getcharged_))
              (Default|HidePowerHint (Variables|Default|GetPlayer%20UI))
              (Variables|Default|Setfirst_use_ false))
            (elif (Variables|Default|Getfirst_charge_use)
              (if (Variables|Default|Getcharged_)
                (Default|HideChargeHint (Variables|Default|GetPlayer%20UI))
                (Variables|Default|Setfirst_charge_use false)))))))))

(fn UpdateWindCD
  (params (dt :type Float%20%28single-precision%29))
  (if (not (Variables|Default|Getwind_ready_))
    (bind _output_get (Variables|Default|Setwind_timer_ (+ dt (Variables|Default|Getwind_timer_))))
    (if (>= _output_get (Variables|Default|Getwind_cooldown_))
      (Variables|Default|Setwind_timer_ 0.0)
      (Variables|Default|Setwind_ready_ true)
      (if (Variables|Default|Getwind_input_down_)
        (Audio|Components|Audio|Play (Variables|Default|GetAudio) 0.0)))))

(fn ToggleinCave
  (params (InCave :type Boolean))
  (bind _directional_light_ (Variables|Default|Getdirectional_light_))
  (bind _lightcomponent (Variables|/Script/Engine.Light|GetLightComponent _directional_light_))
  (Variables|Default|Setin_cave_ InCave)
  (if (not (Variables|Default|Getintuition_mode_))
    (if (Variables|Default|Getin_cave_)
      (Rendering|Components|Light|SetIntensity _lightcomponent 0.0)
      (else
        (Rendering|Components|Light|SetIntensity _lightcomponent (Variables|Default|Getoriginal_intensity_))))))

(fn GetWindPower
  (bind _camera (Variables|Default|GetCamera))
  (bind _returnvalue (Transformation|GetWorldLocation _camera))
  (bind _outhit (Collision|LineTraceByChannel _returnvalue (+ _returnvalue (* (Math|Vector|GetForwardVector _camera) (Variables|Default|Getwind_range_))) "TraceTypeQuery3" false 0 "None"))
  (bind _asbp_ability_orb (Utilities|Casting|CastToBP_AbilityOrb (.hitactor _outhit)))
  (if (Variables|/Game/Blueprints/BP_AbilityOrb.BP_AbilityOrb_C|Getis_activated_ _asbp_ability_orb)
    (bind _output_get (Variables|Default|Sethave_wind_power_ true))
    (Variables|/Game/Blueprints/BP_AbilityOrb.BP_AbilityOrb_C|Setis_claimed_ _asbp_ability_orb _output_get)
    (Variables|Default|Setwind_ready_ false)
    (Default|HideClaimHint (Variables|Default|GetPlayer%20UI))))

(fn SetUI
  (params (PlayerUI :type Player%20UI%20Object%20Reference))
  (Variables|Default|SetPlayer%20UI PlayerUI))