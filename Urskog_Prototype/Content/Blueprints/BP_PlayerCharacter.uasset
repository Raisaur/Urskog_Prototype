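; First-person-style player character with walk, look, jump, hold-to-run and a cooldown-limited wind push ability.
; Wind spawns a Niagara effect at the camera, box-traces forward and applies a velocity-change radial impulse from the actor to physics-simulating hit components.
; Tick advances the cooldown, which starts on a push or empty trace, but not when all hits are non-simulating.
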(event EventBeginPlay
  (Variables|Default|Setwalk_speed_ (Variables|/Script/Engine.CharacterMovementComponent|GetMaxWalkSpeed (Variables|Character|GetCharacterMovement))))

(event Collision|EventActorBeginOverlap
  (params (OtherActor :type Actor%20Object%20Reference)))

(event EventTick
  (params (DeltaSeconds :type Float%20%28single-precision%29))
  (CallFunction|UpdateWindCD DeltaSeconds))

(event Input|ActionEvents|InputActionJump
  (params (Key :type Key%20Structure :default "None"))
  ;[1 1 1] Movement and Camera
  (:Pressed
    (Character|Jump))
  (:Released
    (Character|StopJumping)))

(event Input|ActionEvents|InputActionUseAbility
  (params (Key :type Key%20Structure :default "None"))
  (:Pressed
    (CallFunction|Wind)))

(event Input|ActionEvents|InputActionRun
  (params (Key :type Key%20Structure :default "None"))
  (bind _charactermovement (Variables|Character|GetCharacterMovement))
  ;[1 1 1] Movement and Camera
  (:Pressed
    (Variables|/Script/Engine.CharacterMovementComponent|SetMaxWalkSpeed _charactermovement (Variables|Default|Getrun_speed_)))
  (:Released
    (Variables|/Script/Engine.CharacterMovementComponent|SetMaxWalkSpeed _charactermovement (Variables|Default|Getwalk_speed_))))

(event Input|AxisEvents|InputAxisMoveForward
  (params (AxisValue :type Float%20%28single-precision%29))
  ;[1 1 1] Movement and Camera
  (Pawn|Input|AddMovementInput (Transformation|GetActorForwardVector) AxisValue false))

(event Input|AxisEvents|InputAxisMoveRight
  (params (AxisValue :type Float%20%28single-precision%29))
  ;[1 1 1] Movement and Camera
  (Pawn|Input|AddMovementInput (Transformation|GetActorRightVector) AxisValue false))

(event Input|AxisEvents|InputAxisLookUp
  (params (AxisValue :type Float%20%28single-precision%29))
  ;[1 1 1] Movement and Camera
  (Pawn|Input|AddControllerPitchInput AxisValue))

(event Input|AxisEvents|InputAxisTurn
  (params (AxisValue :type Float%20%28single-precision%29))
  ;[1 1 1] Movement and Camera
  (Pawn|Input|AddControllerYawInput AxisValue))

(fn ConstructionScript)

(fn Wind
  (bind _camera (Variables|Default|GetCamera))
  (bind _returnvalue (Transformation|GetWorldLocation _camera))
  (bind _returnvalue_2 (Transformation|GetWorldRotation _camera))
  (bind _returnvalue_3 (Math|Vector|GetForwardVector _camera))
  ;[1 1 1] pushes all objects in front once
  (if (Variables|Default|Getwind_ready_)
    (Niagara|SpawnSystematLocation "/Game/VFX/WindVFX/VFX_WindPush_System.VFX_WindPush_System" (+ (* _returnvalue_3 5e+01) _returnvalue) (Math|Rotator|MakeRotator (.roll _returnvalue_2) (.pitch _returnvalue_2) (- (.yaw (Transformation|GetWorldRotation (Variables|Collision|GetCapsuleComponent))) 9e+01)))
    (bind (_outhits _returnvalue_4) (Class|KismetSystemLibrary|BoxTraceMultiforObjects _returnvalue (+ _returnvalue (* _returnvalue_3 (Variables|Default|Getwind_range_))) "100.000000,100.000000,100.000000" "0, 0, 0" (Utilities|Array|MakeArray "ObjectTypeQuery1" "ObjectTypeQuery3" "ObjectTypeQuery4") false 0 "None" true))
    (if _returnvalue_4
      (for _array_element _outhits
        (if (Physics|IsSimulatingPhysics (.HitComponent (Collision|BreakHitResult _array_element)) "None")
          (Physics|AddRadialImpulse (.HitComponent (Collision|BreakHitResult _array_element)) (Transformation|GetActorLocation) 5e+03 2e+03 "RIF_Constant" true)
          (Variables|Default|Setwind_ready_ false)))
      (else
        (Variables|Default|Setwind_ready_ false)))))

(fn UpdateWindCD
  (params (dt :type Float%20%28single-precision%29))
  (if (not (Variables|Default|Getwind_ready_))
    (bind _output_get (Variables|Default|Setwind_timer_ (+ dt (Variables|Default|Getwind_timer_))))
    (if (>= _output_get (Variables|Default|Getwind_cooldown_))
      (Variables|Default|Setwind_timer_ 0.0)
      (Variables|Default|Setwind_ready_ true))))