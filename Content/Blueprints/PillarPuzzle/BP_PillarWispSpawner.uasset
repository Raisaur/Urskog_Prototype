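; Spawner actor for the pillar puzzle that keeps a population of BP_PillarWisp actors up to a maximum count.
; It spawns one on BeginPlay if allowed, then Tick accumulates a timer that, after a few seconds, prunes invalid wisps and attempts a refill.
; Spawning happens at the Scene component's transform and clears a CanSpawn flag, which is set again when a wisp leaves the Box overlap.
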(event OnComponentEndOverlap(Box)
  (params (OverlappedComponent :type Primitive%20Component%20Object%20Reference) (OtherActor :type Actor%20Object%20Reference) (OtherComp :type Primitive%20Component%20Object%20Reference) (OtherBodyIndex :type Integer))
  (Utilities|Casting|CastToBP_PillarWisp OtherActor)
  (Variables|Default|Setcan_spawn_ true))

(event EventBeginPlay
  (CallFunction|SpawnWisp))

(event Collision|EventActorBeginOverlap
  (params (OtherActor :type Actor%20Object%20Reference)))

(event EventTick
  (params (DeltaSeconds :type Float%20%28single-precision%29))
  (CallFunction|Timers DeltaSeconds)
  (if (>= (Variables|Default|Gettimer_) 5.0)
    (CallFunction|CheckList)))

(fn ConstructionScript)

(fn SpawnWisp
  (bind _scene (Variables|Default|GetScene))
  (bind _returnvalue (Transformation|GetWorldTransform _scene))
  (if (Variables|Default|Getcan_spawn_)
    ;[1 1 1] Spawn Animation?
    (bind _returnvalue_2 (Game|SpawnActorfromClass "/Game/Blueprints/PillarPuzzle/BP_PillarWisp.BP_PillarWisp_C" (Math|Transform|MakeTransform (.location _returnvalue) (.rotation _returnvalue) "1,1,1") "Undefined" 0 0))
    (Utilities|Array|Add (Variables|Default|Getwisps_) _returnvalue_2)
    (Variables|Default|Setcan_spawn_ false)))

(fn CheckList
  (for (_array_element _array_index) (Variables|Default|Getwisps_)
    (if (not (Utilities|IsValid _array_element))
      (Utilities|Array|RemoveIndex (Variables|Default|Getwisps_) _array_index)))
  (if (< (Utilities|Array|Length (Variables|Default|Getwisps_)) (Variables|Default|Getmax_wisp_ammount_))
    (CallFunction|SpawnWisp)
    (Variables|Default|Settimer_ 0.0)))

(fn Timers
  (params (dt :type Float%20%28single-precision%29))
  (Variables|Default|Settimer_ (+ dt (Variables|Default|Gettimer_)))
  (if (> 0.0 0.0)
    _))