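; BP_WindDoor is a musical puzzle door that opens when its linked pipes are triggered in the correct order.
; On BeginPlay it gives each pipe an index and a self-reference; SendPipe records incoming indices and compares them to CorrectPipeOrder.
; Correct entries light up through scalar parameters in the MP_MusicDoorPuzzle collection, while a mismatch clears the sequence and lights.
; A completed sequence plays the opening sound and skeletal animation and activates Niagara.
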(event EventBeginPlay
  (for (_array_element _array_index) (Variables|Default|Getpipes_)
    (Default|SetPipeIndex _array_element _array_index)
    (Default|SetDoor _array_element self)))

(event Collision|EventActorBeginOverlap
  (params (OtherActor :type Actor%20Object%20Reference)))

(event EventTick
  (params (DeltaSeconds :type Float%20%28single-precision%29)))

(fn ConstructionScript)

(fn SendPipe
  (params (pipe_nr :type Integer))
  (bind _sent_pipe_order_ (Variables|Default|Getsent_pipe_order_))
  (Development|PrintString (Utilities|String|ToString(Integer) pipe_nr))
  (bind (_array_element _array_index) (Utilities|Array|ForEachLoopwithBreak _sent_pipe_order_ :!label _label)
    (:LoopBody
      (if (== _array_element -1)
        (Utilities|Array|SetArrayElem _sent_pipe_order_ _array_index pipe_nr)
        (goto _label Break)))
    (:Completed
      (Variables|Default|Setpuzzle_done_ true)
      (bind (_array_element_2 _array_index_2) (Utilities|Array|ForEachLoopwithBreak (Variables|Default|Getcorrect_pipe_order_) :!label _label_2)
        (:LoopBody
          (if (!= (Utilities|Array|Get(acopy) (Variables|Default|Getsent_pipe_order_) _array_index_2) -1)
            (if (== _array_element_2 (Utilities|Array|Get(acopy) (Variables|Default|Getsent_pipe_order_) _array_index_2))
              (bind _name (CallFunction|GetLightParamaterName _array_index_2))
              (Rendering|Material|SetScalarParameterValue "/Game/Models/MusicDoor/MP_MusicDoorPuzzle.MP_MusicDoorPuzzle" _name 1.0 :!class /Script/Engine.KismetMaterialLibrary)
              (else
                (CallFunction|Reset)
                (Variables|Default|Setpuzzle_done_ false)
                (goto _label_2 Break)))
            (else
              (Variables|Default|Setpuzzle_done_ false))))
        (:Completed
          (if (Variables|Default|Getpuzzle_done_)
            (CallFunction|Open)))))))

(fn Reset
  (bind _sent_pipe_order_ (Variables|Default|Getsent_pipe_order_))
  (for (_ _array_index) _sent_pipe_order_
    (Utilities|Array|SetArrayElem _sent_pipe_order_ _array_index -1)
    (bind _name (CallFunction|GetLightParamaterName _array_index))
    (Rendering|Material|SetScalarParameterValue "/Game/Models/MusicDoor/MP_MusicDoorPuzzle.MP_MusicDoorPuzzle" _name 0.0 :!class /Script/Engine.KismetMaterialLibrary)))

(fn Open
  (Audio|PlaySoundatLocation (Variables|Default|Getdoor_opening_sound_) (Transformation|GetWorldLocation (Variables|Default|GetSkeletalMesh)) "0, 0, 0" 1.0 1.0 0.0 0 0 0)
  (Components|Animation|PlayAnimation (Variables|Default|GetSkeletalMesh) "/Game/Models/MusicDoor/SK_MusicDoor_Anim.SK_MusicDoor_Anim" false)
  (Components|Activation|Activate (Variables|Default|GetNiagara) true))

(fn GetLightParamaterName
  (params (i :type Integer))
  (switch int i
    (:0
      (return (Utilities|Name|MakeLiteralName "Light_01")))
    (:1
      (return (Utilities|Name|MakeLiteralName "Light_02")))
    (:2
      (return (Utilities|Name|MakeLiteralName "Light_03")))
    (:3
      (return (Utilities|Name|MakeLiteralName "Light_04")))
    (:4
      (return (Utilities|Name|MakeLiteralName "Light_05")))))