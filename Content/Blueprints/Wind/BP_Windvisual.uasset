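; BP_Windvisual is a short-lived wind visual actor that destroys itself one second after BeginPlay.
; Each Tick it publishes its location as P1 to the MP_Windballposition material parameter collection, along with two derived points, P2 and P3.
; P2 and P3 start at the spawn location and lerp toward the actor with alphas above one, so they overshoot its current position by different amounts.
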(event EventBeginPlay
  (bind _output_get (Variables|Default|SetP2 (- (Transformation|GetActorLocation) (Math|Vector|MakeVector 0.0 0.0 0.0))))
  (Variables|Default|SetP3 _output_get)
  (Actor|SetLifeSpan 1.0))

(event Collision|EventActorBeginOverlap
  (params (OtherActor :type Actor%20Object%20Reference)))

(event EventTick
  (params (DeltaSeconds :type Float%20%28single-precision%29))
  (bind _returnvalue (Transformation|GetActorLocation))
  (bind _returnvalue_2 (- _returnvalue (Math|Vector|MakeVector 0.0 0.0 0.0)))
  (Rendering|Material|SetVectorParameterValue "/Game/Blueprints/MP_Windballposition.MP_Windballposition" "P1" (Math|Conversions|ToLinearColor(Vector) _returnvalue_2) :!class /Script/Engine.KismetMaterialLibrary)
  (bind _output_get (Variables|Default|SetP2 (Math|Vector|Lerp(Vector) (Variables|Default|GetP2) _returnvalue_2 1.3)))
  (Rendering|Material|SetVectorParameterValue "/Game/Blueprints/MP_Windballposition.MP_Windballposition" "P2" (Math|Conversions|ToLinearColor(Vector) _output_get) :!class /Script/Engine.KismetMaterialLibrary)
  (bind _output_get_2 (Variables|Default|SetP3 (Math|Vector|Lerp(Vector) (Variables|Default|GetP3) _returnvalue_2 1.2)))
  (Rendering|Material|SetVectorParameterValue "/Game/Blueprints/MP_Windballposition.MP_Windballposition" "P3" (Math|Conversions|ToLinearColor(Vector) _output_get_2) :!class /Script/Engine.KismetMaterialLibrary))

(fn ConstructionScript)