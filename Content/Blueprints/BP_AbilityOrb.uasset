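; BP_AbilityOrb is a pickup orb that activates when the player enters its trigger and can then be claimed.
; Tick runs timed lerps on MP_AbilityOrb material parameter collection scalars, first fading out the deactivated look, then raising the claimed effect.
; Finishing activation shows claim text on the UI passed in through GetUI.
; IsClaimed, not set in this Blueprint, starts the claim phase and a one-shot pickup sound.
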(event OnComponentBeginOverlap(Trigger)
  (params (OverlappedComponent :type Primitive%20Component%20Object%20Reference) (OtherActor :type Actor%20Object%20Reference) (OtherComp :type Primitive%20Component%20Object%20Reference) (OtherBodyIndex :type Integer) (bFromSweep :type Boolean) (SweepResult :type Hit%20Result%20Structure%20%28by%20ref%29))
  (Utilities|Casting|CastToBP_PlayerCharacter OtherActor)
  (Variables|Default|Setactivate_ true))

(event EventTick
  (params (DeltaSeconds :type Float%20%28single-precision%29))
  (if (not (Variables|Default|Getdone_))
    (if (Variables|Default|Getis_activated_)
      (if (Variables|Default|Getis_claimed_)
        (bind _output_get (Variables|Default|Settimer_ (+ DeltaSeconds (Variables|Default|Gettimer_))))
        (Rendering|Material|SetScalarParameterValue "/Game/VFX/AbilityOrb/MP_AbilityOrb.MP_AbilityOrb" "OrbClaimed" (Math|Float|Lerp 0.0 6.0 (/ _output_get (Variables|Default|Gettime_to_claim_))) :!class /Script/Engine.KismetMaterialLibrary)
        (Utilities|FlowControl|DoOnce false
          (:Completed
            (Audio|PlaySoundatLocation "/Game/Audio/Ambient/AbilityOrbPickup.AbilityOrbPickup" (Transformation|GetWorldLocation (Variables|Default|GetStaticMesh)) "0, 0, 0" 1.0 1.0 0.0 0 0 0)
            (Variables|Default|Setdone_ (>= (Variables|Default|Gettimer_) (Variables|Default|Gettime_to_claim_))))))
      (elif (Variables|Default|Getactivate_)
        (bind _output_get_2 (Variables|Default|Settimer_ (+ DeltaSeconds (Variables|Default|Gettimer_))))
        (Rendering|Material|SetScalarParameterValue "/Game/VFX/AbilityOrb/MP_AbilityOrb.MP_AbilityOrb" "OrbDectivated" (Math|Float|Lerp 1.0 0.0 (/ _output_get_2 (Variables|Default|Gettime_to_activate))) :!class /Script/Engine.KismetMaterialLibrary)
        (bind _output_get_3 (Variables|Default|Setis_activated_ (>= (Variables|Default|Gettimer_) (Variables|Default|Gettime_to_activate))))
        (if _output_get_3
          (Variables|Default|Settimer_ 0.0)
          (Default|ShowClaimText (Variables|Default|GetPlayer%20UI)))))))

(fn ConstructionScript)

(fn GetUI
  (params (PlayerUI :type Player%20UI%20Object%20Reference))
  (Variables|Default|SetPlayer%20UI PlayerUI))