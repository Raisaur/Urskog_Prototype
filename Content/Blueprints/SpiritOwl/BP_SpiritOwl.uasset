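; Spirit owl that is visible only during the player's intuition mode and flies away once it spots the player.
; Intuition dispatchers from the player character toggle its visibility and a material parameter collection fade.
; Overlapping the fly trigger starts a looping timer that focuses the AI on the player and line-traces during intuition.
; On a hit, a timeline moves it along the Waypoints spline with a hoot, then hides it and spawns an effect.
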(event OnComponentBeginOverlap(FlyTrigger)
  (params (OverlappedComponent :type Primitive%20Component%20Object%20Reference) (OtherActor :type Actor%20Object%20Reference) (OtherComp :type Primitive%20Component%20Object%20Reference) (OtherBodyIndex :type Integer) (bFromSweep :type Boolean) (SweepResult :type Hit%20Result%20Structure%20%28by%20ref%29))
  (bind _asbp_player_character (Utilities|Casting|CastToBP_PlayerCharacter OtherActor))
  (Variables|Default|SetPlayer _asbp_player_character)
  (bind _returnvalue (Utilities|Time|SetTimerbyEvent (delegate Custom|SpotPlayer) 1.0 true)))

(event Custom|IntuitionOn
  ;[1 1 1] Show mesh
  (Rendering|Material|SetScalarParameterValue "/Game/VFX/Intuitionmode/MP_Intuitionmode.MP_Intuitionmode" "Sprit_animal_fade" 1.0 :!class /Script/Engine.KismetMaterialLibrary)
  (Rendering|SetActorHiddenInGame false)
  (Variables|Default|SetIntuitionMode true))

(event Custom|IntuitionOff
  ;[1 1 1] Hide mesh
  (Rendering|Material|SetScalarParameterValue "/Game/VFX/Intuitionmode/MP_Intuitionmode.MP_Intuitionmode" "Sprit_animal_fade" 0.0 :!class /Script/Engine.KismetMaterialLibrary)
  (Rendering|SetActorHiddenInGame true)
  (Variables|Default|SetIntuitionMode false))

(event Custom|SpotPlayer
  (bind _player (Variables|Default|GetPlayer))
  (if (not (Variables|Default|GetIsFlying))
    (Utilities|IsValid _player
      (:Is%20Valid
        (AI|SetFocus (AI|GetAIController self) _player)
        (if (Variables|Default|GetIntuitionMode)
          (bind _canseeplayer (CallFunction|CheckLineOfSight (Variables|Default|GetPlayer)))
          (if _canseeplayer
            (Variables|Default|SetIsFlying true)
            (Utilities|Time|ClearandInvalidateTimerbyHandle (stale OnComponentBeginOverlap(FlyTrigger) _returnvalue))
            (Audio|PlaySoundatLocation "/Game/Audio/Ambient/Great_Grey_Owl_-_QuickSounds_com.Great_Grey_Owl_-_QuickSounds_com" (Transformation|GetActorLocation) "0, 0, 0" 1.0 1.0 0.0 0 0 0)
            (Components|Timeline|SetPlayRate (Variables|Default|GetTimeline_0) (/ 1.0 (Variables|Default|GetDuration)))
            (bind _newtrack_0 (Timeline|Timeline_0 Play)
              (:Update
                (Variables|Default|SetAlpha _newtrack_0)
                (Transformation|SetActorLocationAndRotation (Spline|GetLocationatDistanceAlongSpline (Variables|/Game/Blueprints/SplineMovement/BP_Track.BP_Track_C|GetSpline (Variables|Default|GetWaypoints)) (Math|Float|Lerp 0.0 (Spline|GetSplineLength (Variables|/Game/Blueprints/SplineMovement/BP_Track.BP_Track_C|GetSpline (Variables|Default|GetWaypoints))) (Variables|Default|GetAlpha)) "World") (Spline|GetRotationatDistanceAlongSpline (Variables|/Game/Blueprints/SplineMovement/BP_Track.BP_Track_C|GetSpline (Variables|Default|GetWaypoints)) (Math|Float|Lerp 0.0 (Spline|GetSplineLength (Variables|/Game/Blueprints/SplineMovement/BP_Track.BP_Track_C|GetSpline (Variables|Default|GetWaypoints))) (Variables|Default|GetAlpha)) "World")))
              (:Finished
                (Rendering|SetActorHiddenInGame true)
                (Game|SpawnActorfromClass "/Game/Blueprints/SpiritOwl/BP_SpiritAnimalEffect.BP_SpiritAnimalEffect_C" (Transformation|GetActorTransform) "Undefined" 0 0)))))))))

(event EventBeginPlay
  ;[1 1 1] Act when player enables intuition mode
  (bind _asbp_player_character (Utilities|Casting|CastToBP_PlayerCharacter (Game|GetPlayerCharacter 0)))
  (EventDispatchers|BindEventtoIntuitiononEventDispatcher _asbp_player_character (delegate Custom|IntuitionOn))
  (EventDispatchers|BindEventtoIntuitionOffEventDispatcher _asbp_player_character (delegate Custom|IntuitionOff))
  (Rendering|SetActorHiddenInGame true))

(fn ConstructionScript)

(fn CheckLineOfSight
  (params (Other :type Actor%20Object%20Reference))
  (bind _outhit (Collision|LineTraceForObjects (+ (Transformation|GetActorLocation) "0,100.000000, 0") (Transformation|GetActorLocation Other) (Utilities|Array|MakeArray "ObjectTypeQuery1" "ObjectTypeQuery3") false 0 "Persistent"))
  (return (Components|ComponentHasTag (.HitComponent (Collision|BreakHitResult _outhit)) (Variables|Default|GetPlayerTag))))