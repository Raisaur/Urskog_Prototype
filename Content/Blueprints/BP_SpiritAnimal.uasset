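; BP_SpiritAnimal is an AI-driven spirit animal that appears when the player enables intuition mode and leads toward a target actor.
; It binds to the player character's intuition on/off dispatchers, fading via a scalar in the MP_Intuitionmode parameter collection.
; On activation it teleports to the supplied spawn position and starts AIMoveTo toward Target, printing the result.
; Deactivation fades it out and clears AI focus without explicitly stopping movement; the SetFocus call is unconnected.
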(event Custom|IntuitionOn
  (params (SpawnPosition :type Vector))
  ;[1 1 1] Move to target actor and enable mesh
  (Rendering|Material|SetScalarParameterValue "/Game/VFX/Intuitionmode/MP_Intuitionmode.MP_Intuitionmode" "Sprit_animal_fade" 1.0 :!class /Script/Engine.KismetMaterialLibrary)
  (CallFunction|PlaceAnimalFrontOfPlayer SpawnPosition)
  (bind _movementresult (AI|AIMoveTo self "0, 0, 0" (Variables|Default|GetTarget) 5e+01 false)
    (:OnSuccess
      (Development|PrintString (Utilities|String|EnumtoString _movementresult)))
    (:OnFail
      (Development|PrintString (Utilities|String|EnumtoString _movementresult)))))

(event Custom|IntuitionOff
  ;[1 1 1] Hide mesh
  (Rendering|Material|SetScalarParameterValue "/Game/VFX/Intuitionmode/MP_Intuitionmode.MP_Intuitionmode" "Sprit_animal_fade" 0.0 :!class /Script/Engine.KismetMaterialLibrary)
  (AI|ClearFocus (AI|GetAIController self)))

(event EventBeginPlay
  ;[1 1 1] Act when player enables intuition mode
  (bind _asbp_player_character (Utilities|Casting|CastToBP_PlayerCharacter (Game|GetPlayerCharacter 0)))
  (EventDispatchers|BindEventtoIntuitiononEventDispatcher _asbp_player_character (delegate Custom|IntuitionOn))
  (EventDispatchers|BindEventtoIntuitionOffEventDispatcher _asbp_player_character (delegate Custom|IntuitionOff)))

(fn ConstructionScript)

(fn PlaceAnimalFrontOfPlayer
  (params (PlayerPosition :type Vector))
  (Transformation|SetActorLocation PlayerPosition false true))