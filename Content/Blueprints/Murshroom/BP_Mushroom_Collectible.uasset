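; BP_Mushroom_Collectible is a mushroom pickup that shows a collectible score widget when found.
; Any overlap on its StaticMesh plays MushroomSequence, creates a new Collectibles widget with a reference back to itself, and sets a three-second lifespan on the actor.
; IncrementMushroomsCollected raises the actor's own MushroomsCollected variable and calls the widget's UpdateScore, which the overlap event then calls again.
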(event OnComponentBeginOverlap(StaticMesh)
  (params (OverlappedComponent :type Primitive%20Component%20Object%20Reference) (OtherActor :type Actor%20Object%20Reference) (OtherComp :type Primitive%20Component%20Object%20Reference) (OtherBodyIndex :type Integer) (bFromSweep :type Boolean) (SweepResult :type Hit%20Result%20Structure%20%28by%20ref%29))
  ;[0.9261 0.175 1] Skapar UI när man hittar collectible, och uppdaterar scoren.
  (bind _outactor (Sequencer|Player|CreateLevelSequencePlayer (Variables|Default|GetMushroomSequence)))
  (Sequencer|Player|Play (Variables|/Script/LevelSequence.LevelSequenceActor|GetSequencePlayer _outactor) :!class /Script/MovieScene.MovieSceneSequencePlayer)
  (bind _returnvalue (UserInterface|CreateWidget "/Game/UI/Collectibles.Collectibles_C"))
  (UserInterface|Viewport|AddtoViewport _returnvalue 0)
  (Variables|/Game/UI/Collectibles.Collectibles_C|SetMushroomCollectible _returnvalue self)
  (bind _output_get (Variables|Default|SetCollectibles _returnvalue))
  (CallFunction|IncrementMushroomsCollected)
  (Default|UpdateScore _output_get)
  (Actor|SetLifeSpan 3.0))

(fn ConstructionScript)

(fn IncrementMushroomsCollected
  ;[1 0.3372 0.9979] Here it will add on to the score, everytime a shape is being collected. This is a function.
  (Math|Integer|IncrementInt (Variables|Default|GetMushroomsCollected)
    (:%20%20
      (Default|UpdateScore (Variables|Default|GetCollectibles)))))