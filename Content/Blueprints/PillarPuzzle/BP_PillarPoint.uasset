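; Pillar puzzle target that captures the first BP_PillarWisp to overlap its capsule and spirals it into the point's center.
; On capture it disables the wisp's physics and records its starting distance and angle.
; Tick then shrinks the radius over RotationTime while the per-frame angle step speeds up, placing the wisp by polar coordinates at constant height.
; At zero distance it marks itself Done and calls PuzzleMaster.CheckDone.
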(event OnComponentBeginOverlap(Capsule)
  (params (OverlappedComponent :type Primitive%20Component%20Object%20Reference) (OtherActor :type Actor%20Object%20Reference) (OtherComp :type Primitive%20Component%20Object%20Reference) (OtherBodyIndex :type Integer) (bFromSweep :type Boolean) (SweepResult :type Hit%20Result%20Structure%20%28by%20ref%29))
  (bind _asbp_pillar_wisp (Utilities|Casting|CastToBP_PillarWisp OtherActor))
  (if (not (Utilities|IsValid (Variables|Default|Gettarget_wisp_)))
    (CallFunction|SetStartValues _asbp_pillar_wisp)))

(event EventBeginPlay)

(event Collision|EventActorBeginOverlap
  (params (OtherActor :type Actor%20Object%20Reference)))

(event EventTick
  (params (DeltaSeconds :type Float%20%28single-precision%29))
  (if (Variables|Default|Gethas_wisp_)
    (if (not (Variables|Default|Getdone_))
      (Variables|Default|Settimer_ (+ DeltaSeconds (Variables|Default|Gettimer_)))
      (CallFunction|SetNewAngle)
      (CallFunction|SetNewDistance)
      (CallFunction|SetNewPosition))))

(fn ConstructionScript)

(fn SetStartValues
  (params (Wisp :type BP%20Pillar%20Wisp%20Object%20Reference))
  (bind _defaultsceneroot (Variables|Default|GetDefaultSceneRoot))
  (bind _returnvalue (Transformation|GetWorldLocation _defaultsceneroot))
  (bind _output_get (Variables|Default|Settarget_wisp_ Wisp))
  (Variables|Default|Setstart_velocity_ (Transformation|GetVelocity _output_get))
  (Physics|SetSimulatePhysics (Variables|/Game/Blueprints/PillarPuzzle/BP_PillarWisp.BP_PillarWisp_C|GetSphere _output_get) false)
  (bind _output_get_2 (Variables|Default|Setstart_distance_ (Math|Vector|Distance(Vector) _returnvalue (Transformation|GetActorLocation _output_get))))
  (Variables|Default|Setdistance_ _output_get_2)
  (bind _angle (CallFunction|GetAngle _returnvalue (Transformation|GetActorLocation _output_get)))
  (bind _output_get_3 (Variables|Default|Setangle_ _angle))
  (Variables|Default|Sethas_wisp_ true)
  (Development|PrintString (Utilities|String|ToString(Float) _output_get_3)))

(fn SetNewDistance
  (bind _output_get (Variables|Default|Setdistance_ (Math|Float|Lerp (Variables|Default|Getstart_distance_) 0.0 (/ (Variables|Default|Gettimer_) (Variables|Default|Getrotation_time_)))))
  (bind _output_get_2 (Variables|Default|Setdone_ (<= _output_get 0.0)))
  (if _output_get_2
    (Default|CheckDone (Variables|Default|Getpuzzle_master_))))

(fn GetAngle
  (params (vector%20a :type Vector) (vector%20b :type Vector))
  (return (Class|KismetMathLibrary|DegAtan2 (- (.y vector%20b) (.y vector%20a)) (- (.x vector%20b) (.x vector%20a)))))

(fn SetNewPosition
  (bind _angle_ (Variables|Default|Getangle_))
  (bind _distance_ (Variables|Default|Getdistance_))
  (bind _target_wisp_ (Variables|Default|Gettarget_wisp_))
  (bind _defaultsceneroot (Variables|Default|GetDefaultSceneRoot))
  (bind _returnvalue (Transformation|GetWorldLocation _defaultsceneroot))
  (Transformation|SetActorLocation _target_wisp_ (Math|Vector|MakeVector (+ (* (Math|Trig|Cos(Degrees) _angle_) _distance_) (.x _returnvalue)) (+ (* _distance_ (Math|Trig|Sin(Degrees) _angle_)) (.y _returnvalue)) (.z (Transformation|GetActorLocation _target_wisp_))) false false))

(fn SetNewAngle
  (if (> (+ (Variables|Default|Getangle_) (Math|Float|Lerp 1.0 4.0 (/ (Variables|Default|Gettimer_) (Variables|Default|Getrotation_time_)))) 359.0)
    (Variables|Default|Setangle_ 0.0)
    (else
      (Variables|Default|Setangle_ (+ (Variables|Default|Getangle_) (Math|Float|Lerp 1.0 4.0 (/ (Variables|Default|Gettimer_) (Variables|Default|Getrotation_time_))))))))