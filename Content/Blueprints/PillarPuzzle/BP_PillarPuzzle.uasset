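; Pillar puzzle master that reveals an intuition guide, then releases an owl and clears fog on completion.
; It registers itself with each point in PointList, and CheckDone spawns the guide effect at the destructible once all are done.
; Finish runs once, enabling physics on the destructible and spawning a track-following owl with dust and sounds.
; Tick then fades fog through a material parameter collection and disables the fog collider's collision.
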(event EventBeginPlay
  (for _array_element (Variables|Default|Getpoint_list_)
    (Variables|/Game/Blueprints/PillarPuzzle/BP_PillarPoint.BP_PillarPoint_C|Setpuzzle_master_ _array_element self)))

(event Collision|EventActorBeginOverlap
  (params (OtherActor :type Actor%20Object%20Reference)))

(event EventTick
  (params (DeltaSeconds :type Float%20%28single-precision%29))
  (if (Variables|Default|Getremove_fog_)
    (Variables|Default|Settimer_ (+ DeltaSeconds (Variables|Default|Gettimer_)))
    (CallFunction|SetFogOpacity)))

(fn ConstructionScript)

(fn CheckDone
  (bind _array_element (Utilities|Array|ForEachLoopwithBreak (Variables|Default|Getpoint_list_) :!label _label)
    (:LoopBody
      (bind _output_get (Variables|Default|Setdone_ (Variables|/Game/Blueprints/PillarPuzzle/BP_PillarPoint.BP_PillarPoint_C|Getdone_ _array_element)))
      (if (not _output_get)
        (goto _label Break)))
    (:Completed
      (if (Variables|Default|Getdone_)
        (bind _returnvalue (Niagara|SpawnSystematLocation "/Game/VFX/Intuitionmode/VFX_IntuitionModeGuide_System.VFX_IntuitionModeGuide_System" (Transformation|GetWorldLocation (Variables|Default|GetDestructible)) "0, 0, 0" "1.000000,1.000000,1.000000" false))
        (Variables|Default|Setintuition_effect_ _returnvalue)))))

(fn Finish
  (bind _destructible (Variables|Default|GetDestructible))
  (bind _returnvalue (Transformation|GetWorldTransform _destructible))
  (if (not (Variables|Default|Getfinished_))
    (Components|DestroyComponent (Variables|Default|Getintuition_effect_))
    (Physics|SetSimulatePhysics (Variables|Default|GetDestructible) true)
    (Variables|Default|Setremove_fog_ true)
    (Audio|PlaySoundatLocation "/Game/Audio/Ambient/Great_Grey_Owl_-_QuickSounds_com.Great_Grey_Owl_-_QuickSounds_com" (Transformation|GetWorldLocation (Variables|Default|GetCylinder1)) "0, 0, 0" 1.0 1.0 0.0 0 0 0)
    (bind _returnvalue_2 (Game|SpawnActorfromClass "/Game/Blueprints/SplineMovement/BP_PillarOwl.BP_PillarOwl_C" (Math|Transform|MakeTransform (.location _returnvalue) "0,-90.000000, 0" "1,1,1") "Undefined" 0 0))
    (Variables|/Game/Blueprints/SplineMovement/BP_PillarOwl.BP_PillarOwl_C|SetActivateBird _returnvalue_2 true)
    (Variables|/Game/Blueprints/SplineMovement/BP_PillarOwl.BP_PillarOwl_C|SetTrackRef _returnvalue_2 (Variables|Default|Getowl_track_))
    (Default|Start _returnvalue_2)
    (Niagara|SpawnSystematLocation "/Game/Blueprints/RollingLog/VFX_Dust_System.VFX_Dust_System" (.location _returnvalue))
    (Audio|SpawnSoundatLocation "/Game/Audio/Ambient/IntuitionHint.IntuitionHint" (.location _returnvalue) "0, 0, 0" 0.3 1.0 0.0 0 0)
    (Variables|Default|Setfinished_ true)))

(fn SetFogOpacity
  (Rendering|Material|SetScalarParameterValue "/Game/VFX/CloudsAndFog/MP_Lastpillar.MP_Lastpillar" "Opacity" (Math|Float|Lerp 1.0 0.0 (/ (Variables|Default|Gettimer_) (Variables|Default|Getremove_fog_time_))) :!class /Script/Engine.KismetMaterialLibrary)
  (if (>= (Variables|Default|Gettimer_) (Variables|Default|Getremove_fog_time_))
    (Collision|SetCollisionEnabled (Variables|/Script/Engine.StaticMeshActor|GetStaticMeshComponent (Variables|Default|Getfog_collider_)) "NoCollision")
    (Variables|Default|Setremove_fog_ false)))