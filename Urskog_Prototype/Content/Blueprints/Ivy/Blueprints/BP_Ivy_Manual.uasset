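; BP_Ivy_Manual is an ivy actor that builds a tapering vine of meshes along its spline.
; The construction script adds a spline mesh between each pair of neighboring points, picking one of three static meshes with an unseeded random roll.
; Each segment's end scale shrinks from its start scale by point count and ScaleMult, and carries into the next segment.
; The event graph has no logic.
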(event EventBeginPlay)

(event Collision|EventActorBeginOverlap
  (params (OtherActor :type Actor%20Object%20Reference)))

(event EventTick
  (params (DeltaSeconds :type Float%20%28single-precision%29)))

(fn ConstructionScript
  (bind _spline (Variables|Default|GetSpline))
  (for _index (range 0 (- (Spline|GetNumberOfSplinePoints _spline) 2))
    (bind _returnvalue (AddComponent|AddSplineMeshComponent false))
    (Variables|Default|SetReturnStaticMesh _returnvalue)
    (switch int (Math|Random|RandomIntegerinRange 1 3)
      (:1
        (Components|StaticMesh|SetStaticMesh (Variables|Default|GetReturnStaticMesh) (Variables|Default|GetStaticMesh_0)))
      (:2
        (Components|StaticMesh|SetStaticMesh (Variables|Default|GetReturnStaticMesh) (Variables|Default|GetStaticMesh_1)))
      (:3
        (Components|StaticMesh|SetStaticMesh (Variables|Default|GetReturnStaticMesh) (Variables|Default|GetStaticMesh_2))))
    (Transformation|AttachComponentToComponent _returnvalue (Variables|Default|GetDefaultSceneRoot) "None" "KeepRelative" "KeepRelative" "KeepRelative" true)
    (SplineMesh|SetStartandEnd _returnvalue (.Location (Spline|GetLocationandTangentatSplinePoint _spline _index "Local")) (.Tangent (Spline|GetLocationandTangentatSplinePoint _spline _index "Local")) (.Location (Spline|GetLocationandTangentatSplinePoint _spline (+ _index 1) "Local")) (.Tangent (Spline|GetLocationandTangentatSplinePoint _spline (+ _index 1) "Local")) true :!class /Script/Engine.SplineMeshComponent)
    (SplineMesh|SetStartScale (Variables|Default|GetReturnStaticMesh) (Math|Vector2D|MakeVector2D (Variables|Default|GetScale%20point) (Variables|Default|GetScale%20point)) true :!class /Script/Engine.SplineMeshComponent)
    (Variables|Default|SetScale%20point (* (Variables|Default|GetScale_Mult) (- (Variables|Default|GetScale%20point) (/ 1.0 (Math|Conversions|ToFloat(Integer) (Spline|GetNumberOfSplinePoints (Variables|Default|GetSpline)))))))
    (SplineMesh|SetEndScale (Variables|Default|GetReturnStaticMesh) (Math|Vector2D|MakeVector2D (Variables|Default|GetScale%20point) (Variables|Default|GetScale%20point)) true :!class /Script/Engine.SplineMeshComponent)))