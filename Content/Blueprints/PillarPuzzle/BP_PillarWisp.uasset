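; BP_PillarWisp is a wisp actor, filed under the pillar puzzle, that shrinks with each hit until it is destroyed.
; BeginPlay fills its hit counter from MaxHits, while OnSpawn sets it to one more than that.
; OnHit decrements the counter, then either destroys the actor or lowers Scale and multiplies the Sphere's current world scale by it, so shrinking compounds.
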(event EventBeginPlay
  (Variables|Default|Sethits_left_ (Variables|Default|Getmax_hits_)))

(event Collision|EventActorBeginOverlap
  (params (OtherActor :type Actor%20Object%20Reference)))

(event EventTick
  (params (DeltaSeconds :type Float%20%28single-precision%29)))

(fn ConstructionScript)

(fn OnSpawn
  (Variables|Default|Sethits_left_ (+ (Variables|Default|Getmax_hits_) 1)))

(fn OnHit
  (bind _sphere (Variables|Default|GetSphere))
  (bind _output_get (Variables|Default|Sethits_left_ (- (Variables|Default|Gethits_left_) 1)))
  (if (<= _output_get 0)
    (Actor|DestroyActor)
    (else
      (Variables|Default|Setscale_ (- (Variables|Default|Getscale_) 0.1))
      (Transformation|SetWorldScale3D _sphere (* (Transformation|GetWorldScale _sphere) (Variables|Default|Getscale_))))))